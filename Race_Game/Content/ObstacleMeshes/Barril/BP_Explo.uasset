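; BP_Explo plays a Niagara explosion effect at an ExplodingBarrel that has exploded.
; BeginPlay loops over all ExplodingBarrel actors with an empty body, so Tick reads only the loop's last element.
; While that barrel's HasExploded is true, Tick prints it, sets AnimationPlaying and spawns the effect every frame, as the flag is never checked.
; Unconnected nodes for actor lookup, attached spawning and component destruction never run.
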(event `self.ReceiveTick`
  (params (DeltaSeconds :type "Float (single-precision)"))
  (`/Engine/EditorBlueprintResources/StandardMacros.IsValid` (stale `self.ReceiveBeginPlay` _array_element)
    (:`Is Valid`
      (bind _bhasexploded (`ExplodingBarrel.bHasExploded` (stale `self.ReceiveBeginPlay` _array_element)))
      (if _bhasexploded
        (`KismetSystemLibrary.PrintString` (`KismetStringLibrary.Conv_BoolToString` _bhasexploded))
        (set `self.AnimationPlaying` true)
        (`NiagaraFunctionLibrary.SpawnSystemAtLocation` (`self.Niagara`) (`SceneComponent.K2_GetComponentLocation` (`Actor.RootComponent` (stale `self.ReceiveBeginPlay` _array_element))))))))

(event `self.ReceiveBeginPlay`
  (bind _outactors (`GameplayStatics.GetAllActorsOfClass` "/Script/Race_Game.ExplodingBarrel"))
  (for _array_element _outactors
    _))