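; BP_Timer is a box trigger that starts and ends lap and race timing across three laps in a driving game.
; Each overlap calls start or end events on the cached BP_VehicleAdvPlayerController, with booleans and DoOnce nodes tracking each lap's state.
; The second and third stages require the previous stage to have ended and BP_FinishLane to flag that lap end; that actor is looked up every Tick.
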(event `self.ReceiveActorBeginOverlap`
  (params (OtherActor :type "Actor Object Reference")))

(event `self.ReceiveBeginPlay`
  (bind _asbp_vehicle_adv_player_controller (cast `/Game/VehicleTemplate/Blueprints/BP_VehicleAdvPlayerController` (`GameplayStatics.GetPlayerController` 0)))
  (set `self.As BP Vehicle Adv Player Controller` _asbp_vehicle_adv_player_controller))

(event `self.Box.OnComponentBeginOverlap`
  (params (OverlappedComponent :type "PrimitiveComponent Object Reference") (OtherActor :type "Actor Object Reference") (OtherComp :type "PrimitiveComponent Object Reference") (OtherBodyIndex :type Integer) (bFromSweep :type Boolean) (SweepResult :type "HitResult Structure (by ref)"))
  (bind _as_bp_vehicle_adv_player_controller (`self.As BP Vehicle Adv Player Controller`))
  (bind _as_bp_vehicle_adv_player_controller_2 (`self.As BP Vehicle Adv Player Controller`))
  (bind _as_bp_vehicle_adv_player_controller_3 (`self.As BP Vehicle Adv Player Controller`))
  (`|ExecutionSequence`
    (:`then_0`
      (if (`self.RaceStarted`)
        (`/Game/VehicleTemplate/Blueprints/BP_VehicleAdvPlayerController.End Lap` _as_bp_vehicle_adv_player_controller_3)
        (`/Game/VehicleTemplate/Blueprints/BP_VehicleAdvPlayerController.End Race` _as_bp_vehicle_adv_player_controller_3)
        (set `self.RaceEnd` true)
        (else
          (`/Game/VehicleTemplate/Blueprints/BP_VehicleAdvPlayerController.start Lap` _as_bp_vehicle_adv_player_controller_3)
          (`/Engine/EditorBlueprintResources/StandardMacros.DoOnce` false
            (:`Completed`
              (`/Game/VehicleTemplate/Blueprints/BP_VehicleAdvPlayerController.Start Race` _as_bp_vehicle_adv_player_controller_3)
              (set `self.RaceStarted` true))))))
    (:`then_1`
      (if (`/Game/BP/BP_FinishLane.FirstLapEnd` (stale `self.ReceiveTick` _returnvalue))
        (if (`self.RaceEnd`)
          (if (`self.RaceStarted2`)
            (`/Game/VehicleTemplate/Blueprints/BP_VehicleAdvPlayerController.End Lap 2` _as_bp_vehicle_adv_player_controller_2)
            (`/Game/VehicleTemplate/Blueprints/BP_VehicleAdvPlayerController.End Race2` _as_bp_vehicle_adv_player_controller_2)
            (set `self.Race2End` true)
            (else
              (`/Game/VehicleTemplate/Blueprints/BP_VehicleAdvPlayerController.Start Lap 2` _as_bp_vehicle_adv_player_controller_2)
              (`/Engine/EditorBlueprintResources/StandardMacros.DoOnce` false
                (:`Completed`
                  (`/Game/VehicleTemplate/Blueprints/BP_VehicleAdvPlayerController.Start Race2` _as_bp_vehicle_adv_player_controller_2)
                  (set `self.RaceStarted2` true))))))))
    (:`then_2`
      (if (`/Game/BP/BP_FinishLane.SecondLapEnd` (stale `self.ReceiveTick` _returnvalue))
        (if (`self.Race2End`)
          (if (`self.Race Started 3`)
            (`/Game/VehicleTemplate/Blueprints/BP_VehicleAdvPlayerController.End Lap3` _as_bp_vehicle_adv_player_controller)
            (`/Game/VehicleTemplate/Blueprints/BP_VehicleAdvPlayerController.End Race3` _as_bp_vehicle_adv_player_controller)
            (set `self.Race3End` true)
            (else
              (`/Game/VehicleTemplate/Blueprints/BP_VehicleAdvPlayerController.Start Lap3` _as_bp_vehicle_adv_player_controller)
              (`/Engine/EditorBlueprintResources/StandardMacros.DoOnce` false
                (:`Completed`
                  (`/Game/VehicleTemplate/Blueprints/BP_VehicleAdvPlayerController.Start Race3` _as_bp_vehicle_adv_player_controller)
                  (set `self.Race Started 3` true))))))))))

(event `self.ReceiveTick`
  (params (DeltaSeconds :type "Float (single-precision)"))
  (bind _returnvalue (`GameplayStatics.GetActorOfClass` "/Game/BP/BP_FinishLane.BP_FinishLane_C")))

(fn `UserConstructionScript`)