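; BP_FinishLane is a three-lap finish line for BP_SportsCar_Pawn, with three trigger boxes that start with collision disabled.
; Tick polls the car's checkpoint count, enabling each box only at its exact threshold (6, 13 or 20).
; Reaching a threshold also sets that lap's flag, before any overlap.
; Only the first box has an overlap handler, which increments NbLoop when the car enters.
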(event `self.ReceiveBeginPlay`
  ;[1 1 1] Desactive collision start
  (`|ExecutionSequence`
    (:`then_0`
      (`PrimitiveComponent.SetCollisionEnabled` (`self.Box`) "NoCollision"))
    (:`then_1`
      (`PrimitiveComponent.SetCollisionEnabled` (`self.Box1`) "NoCollision"))
    (:`then_2`
      (`PrimitiveComponent.SetCollisionEnabled` (`self.Box2`) "NoCollision"))))

(event `self.Box.OnComponentBeginOverlap`
  (params (OverlappedComponent :type "PrimitiveComponent Object Reference") (OtherActor :type "Actor Object Reference") (OtherComp :type "PrimitiveComponent Object Reference") (OtherBodyIndex :type Integer) (bFromSweep :type Boolean) (SweepResult :type "HitResult Structure (by ref)"))
  ;[1 1 1] Augmente Nombre de tour effectué
  (cast `/Game/VehicleTemplate/Blueprints/SportsCar/BP_SportsCar_Pawn` OtherActor)
  (set `self.Nb_Loop` (+ (`self.Nb_Loop`) 1.0)))

(event `self.ReceiveTick`
  (params (DeltaSeconds :type "Float (single-precision)"))
  (bind _box (`self.Box`))
  (bind _box1 (`self.Box1`))
  (bind _box2 (`self.Box2`))
  ;[1 1 1] Active collision si condition est TRUE
  (bind _returnvalue (`GameplayStatics.GetActorOfClass` "/Game/VehicleTemplate/Blueprints/SportsCar/BP_SportsCar_Pawn.BP_SportsCar_Pawn_C"))
  (`|ExecutionSequence`
    (:`then_0`
      (if (== (`/Game/VehicleTemplate/Blueprints/SportsCar/BP_SportsCar_Pawn.NB_CheckPointPassed` _returnvalue) 6.0)
        (`|ExecutionSequence`
          (:`then_0`
            (`PrimitiveComponent.SetCollisionEnabled` _box "QueryAndPhysics"))
          (:`then_1`
            (if true
              (set `self.FirstLapEnd` true))))
        (else
          (`PrimitiveComponent.SetCollisionEnabled` _box "NoCollision"))))
    (:`then_1`
      (if (== (`/Game/VehicleTemplate/Blueprints/SportsCar/BP_SportsCar_Pawn.NB_CheckPointPassed` _returnvalue) 13.0)
        (`|ExecutionSequence`
          (:`then_0`
            (`PrimitiveComponent.SetCollisionEnabled` _box1 "QueryAndPhysics"))
          (:`then_1`
            (if true
              (set `self.SecondLapEnd` true))))
        (else
          (`PrimitiveComponent.SetCollisionEnabled` _box1 "NoCollision"))))
    (:`then_2`
      (if (== (`/Game/VehicleTemplate/Blueprints/SportsCar/BP_SportsCar_Pawn.NB_CheckPointPassed` _returnvalue) 20.0)
        (`|ExecutionSequence`
          (:`then_0`
            (`PrimitiveComponent.SetCollisionEnabled` _box2 "QueryAndPhysics"))
          (:`then_1`
            (if true
              (set `self.ThirdLap` true))))
        (else
          (`PrimitiveComponent.SetCollisionEnabled` _box2 "NoCollision"))))))

(fn `UserConstructionScript`)